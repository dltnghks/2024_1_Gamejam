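; Pirate enemy character that moves toward a Destination and switches to pistol combat when it sees the player.
; PawnSensing stops movement, sets IsCombat and plays an attached aiming sound.
; In combat, Tick turns the pirate toward the player and counts to AimTime, then silences the sound and briefly pulses IsShoot.
; Latent Delays in Tick time the pulse and combat exit; otherwise Tick issues AIMoveTo.
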(event `self.ReceiveTick`
  (params (DeltaSeconds :type "Float (single-precision)"))
  (if (`self.IsCombat`)
    (set `self.CountTime` (+ (`self.CountTime`) DeltaSeconds))
    (if (>= (`self.CountTime`) (`self.AimTime`))
      (`AudioComponent.Stop` (`self.AimedSound`))
      (set `self.IsShoot` true)
      (set `self.CountTime` 0.0)
      (`KismetSystemLibrary.Delay` 0.5)
      (set `self.IsShoot` false))
    (`self.LookPlayer`)
    (`KismetSystemLibrary.Delay` 4.3)
    (set `self.IsCombat` false)
    (else
      (`|AIMoveTo` self (`self._destination`) null
        (:`OnSuccess`
          _)
        (:`OnFail`
          _))
      (`KismetSystemLibrary.Delay` (`KismetMathLibrary.RandomFloatInRange` 1.0 3.0)))))

(event `self.PawnSensing.OnSeePawn`
  (params (Pawn :type "Pawn Object Reference"))
  (if (`self.IsCombat`)
    _
    (elif (== Pawn (`GameplayStatics.GetPlayerPawn` 0))
      (set `self.IsCombat` true)
      (`Controller.StopMovement` (`self.GetController`))
      (bind _returnvalue (`GameplayStatics.SpawnSoundAttached` "/Game/Assets/Sound/Pistol/S_AimedPistol.S_AimedPistol" (`self.RootComponent`) "None" (0.0 0.0 0.0) (struct) "KeepRelativeOffset" false 1.0 1.0 0.0 null null))
      (set `self.AimedSound` _returnvalue))))

(fn `LookPlayer`
  (`self.K2_SetActorRotation` (`KismetMathLibrary.FindLookAtRotation` (`self.K2_GetActorLocation`) (`self.K2_GetActorLocation` (`GameplayStatics.GetPlayerPawn` 0)))))

(fn `UserConstructionScript`)